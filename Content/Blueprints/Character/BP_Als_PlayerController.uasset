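; ALS player controller that sets up the local player's UI input mapping, HUD and overlay mode menu.
; Input actions drive overlay selection, UI toggle and slow motion; all but previous-overlay call empty functions, apparently overridden by the script module named in GetModuleName.
; The original Blueprint logic for those actions remains as disconnected, unexecuted nodes.
; A time dilation helper applies changes only in standalone games.
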(event Input|EnhancedActionEvents|EnhancedInputActionIA_Als_OverlayModeMenu
  (params (ActionValue :type Boolean) (ElapsedSeconds :type Float%20%28double-precision%29) (TriggeredSeconds :type Float%20%28double-precision%29) (InputAction :type Input%20Action%20Object%20Reference :default "/ALS/ALSExtras/Data/Input/IA_Als_OverlayModeMenu.IA_Als_OverlayModeMenu"))
  (:Triggered
    (CallFunction|OnOverlayModeTrigger ActionValue)))

(event Input|EnhancedActionEvents|EnhancedInputActionIA_Als_NextOverlayMode
  (params (ActionValue :type Boolean) (ElapsedSeconds :type Float%20%28double-precision%29) (TriggeredSeconds :type Float%20%28double-precision%29) (InputAction :type Input%20Action%20Object%20Reference :default "/ALS/ALSExtras/Data/Input/IA_Als_NextOverlayMode.IA_Als_NextOverlayMode"))
  (:Triggered
    (CallFunction|OnNextOverlayMode)))

(event Input|EnhancedActionEvents|EnhancedInputActionIA_Als_PreviousOverlayMode
  (params (ActionValue :type Boolean) (ElapsedSeconds :type Float%20%28double-precision%29) (TriggeredSeconds :type Float%20%28double-precision%29) (InputAction :type Input%20Action%20Object%20Reference :default "/ALS/ALSExtras/Data/Input/IA_Als_PreviousOverlayMode.IA_Als_PreviousOverlayMode"))
  (:Triggered
    (if (UserInterface|Viewport|IsinViewport (Variables|State|GetOverlayModeMenuWidget))
      (Default|SelectPreviousOverlayMode (Variables|State|GetOverlayModeMenuWidget)))))

(event Input|EnhancedActionEvents|EnhancedInputActionIA_Als_ToggleUI
  (params (ActionValue :type Boolean) (ElapsedSeconds :type Float%20%28double-precision%29) (TriggeredSeconds :type Float%20%28double-precision%29) (InputAction :type Input%20Action%20Object%20Reference :default "/ALS/ALSExtras/Data/Input/IA_Als_ToggleUI.IA_Als_ToggleUI"))
  (:Triggered
    (CallFunction|OnToggleUI)))

(event Input|EnhancedActionEvents|EnhancedInputActionIA_Als_Slomo
  (params (ActionValue :type Boolean) (ElapsedSeconds :type Float%20%28double-precision%29) (TriggeredSeconds :type Float%20%28double-precision%29) (InputAction :type Input%20Action%20Object%20Reference :default "/ALS/ALSExtras/Data/Input/IA_Als_Slomo.IA_Als_Slomo"))
  (:Triggered
    (CallFunction|OnSlomo)))

(event EventBeginPlay
  (if (Pawn|IsLocalController)
    (Input|SetInputModeGameOnly self)
    (Input|AddMappingContext (PlayerController|LocalPlayerSubsystems|GetEnhancedInputLocalPlayerSubsystem) "/ALS/ALSExtras/Data/Input/IMC_Als_UI.IMC_Als_UI" 0 "(bIgnoreAllPressedKeysUntilRelease=True,bForceImmediately=False)")
    (bind _returnvalue (UserInterface|CreateWidget "/ALS/ALSExtras/UI/W_Als_Hud.W_Als_Hud_C" self))
    (UserInterface|Viewport|AddtoViewport _returnvalue 0)
    (bind _returnvalue_2 (UserInterface|CreateWidget "/ALS/ALSExtras/UI/W_Als_OverlayModeMenu.W_Als_OverlayModeMenu_C" self))
    (Variables|State|SetOverlayModeMenuWidget _returnvalue_2)))

(fn ConstructionScript)

(fn SetGlobalTimeDilation
  (params (Time%20Dilation :type Float%20%28double-precision%29))
  (if (Class|KismetSystemLibrary|IsStandalone)
    (Utilities|Time|SetGlobalTimeDilation Time%20Dilation)))

(fn OnOverlayModeTrigger
  (params (Value :type Boolean)))

(fn OnNextOverlayMode)

(fn OnToggleUI)

(fn OnSlomo)

(fn GetModuleName
  (return "GameWorld.Character.AlsPlayerController"))